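; BP_EnigmaLight is a puzzle light that blinks a color sequence and shows whether the puzzle is solved or failed.
; DisplayColor recursively consumes the color array, lighting purple, yellow or blue, toggling intensity between delays, then turning white when empty.
; Victory turns the light green and sets a flag that stops replays through StartDisplayColor.
; Wrong turns it red, waits briefly, then restarts the display.
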(event Custom|Display%20Color
  (params (NewParam :type Array%20of%20E_MushroomColor%20Enums :default "NewEnumerator0"))
  (if (not (Utilities|Array|IsEmpty NewParam))
    (switch Utilities|FlowControl|Switch|SwitchonE_MushroomColor (Utilities|Array|Get(acopy) NewParam)
      (:NewEnumerator0
        (Rendering|Components|Light|SetLightColor (Variables|Default|GetPointLight) "(R=1.000000,G=0.000000,B=0.750000,A=1.000000)" true))
      (:NewEnumerator1
        (Rendering|Components|Light|SetLightColor (Variables|Default|GetPointLight) "(R=1.000000,G=0.973409,B=0.000000,A=1.000000)" true))
      (:NewEnumerator2
        (Rendering|Components|Light|SetLightColor (Variables|Default|GetPointLight) "(R=0.000000,G=0.974654,B=1.000000,A=1.000000)" true)))
    (Utilities|FlowControl|Delay 1.0)
    (Rendering|Components|Light|SetIntensity (Variables|Default|GetPointLight) 0.0)
    (Utilities|FlowControl|Delay 1.0)
    (Rendering|Components|Light|SetIntensity (Variables|Default|GetPointLight) 5e+03)
    (Utilities|Array|RemoveIndex NewParam)
    (CallFunction|DisplayColor NewParam)
    (else
      (Rendering|Components|Light|SetLightColor (Variables|Default|GetPointLight) "(R=1.000000,G=1.000000,B=1.000000,A=1.000000)" true))))

(event Custom|StartDisplayColor
  (if (not (Variables|Default|GetWiin))
    (CallFunction|DisplayColor (Variables|Default|GetColorArray))))

(event Custom|Wrong
  (Rendering|Components|Light|SetLightColor (Variables|Default|GetPointLight) "(R=1.000000,G=0.030088,B=0.000000,A=1.000000)" true)
  (Utilities|FlowControl|Delay 2.0)
  (CallFunction|StartDisplayCOlor))

(event Custom|Victory
  (Variables|Default|SetWiin true)
  (Rendering|Components|Light|SetLightColor (Variables|Default|GetPointLight) "(R=0.000000,G=1.000000,B=0.062372,A=1.000000)" true))

(fn ConstructionScript)