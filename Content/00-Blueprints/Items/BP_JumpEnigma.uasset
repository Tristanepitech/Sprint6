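; Colored mushroom element of a jump puzzle that reports its Purple, Yellow or Blue color when something overlaps its sphere.
; After a short delay, an overlap calls Jumped with that color, flashes the point light white, plays a boing and runs a timeline scaling the mushroom.
; Victory turns the light green and disables further triggers.
; WRONG shows red and blocks triggers briefly before restoring the color.
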(event OnComponentBeginOverlap(Sphere)
  (params (OverlappedComponent :type Primitive%20Component%20Object%20Reference) (OtherActor :type Actor%20Object%20Reference) (OtherComp :type Primitive%20Component%20Object%20Reference) (OtherBodyIndex :type Integer) (bFromSweep :type Boolean) (SweepResult :type Hit%20Result%20Structure%20%28by%20ref%29))
  (if (not (Variables|Default|GetWiin))
    (if (not (Variables|Default|GetWrongAnime))
      (Utilities|FlowControl|Delay 0.2)
      (Default|CallJumped (Variables|Default|GetE_Color))
      (Rendering|Components|Light|SetLightColor (Variables|Default|GetPointLight) "(R=1.000000,G=1.000000,B=1.000000,A=1.000000)" true)
      (Audio|PlaySound2D "/Game/02-Musics_SFX/Mushroom/boing-2-44164.boing-2-44164" 1.0 1.0 0.0 0 0)
      (Utilities|FlowControl|Sequence
        (:then_0
          (bind _newtrack_0 (Timeline|Timeline PlayFromStart)
            (:Update
              (Transformation|SetWorldScale3D (Variables|Default|GetMushRoom) (Math|Vector|MakeVector _newtrack_0 _newtrack_0 _newtrack_0)))))
        (:then_1
          (Utilities|FlowControl|Delay 0.4)
          (CallFunction|SetColor))))))

(event Custom|SetColor
  (switch Utilities|FlowControl|Switch|SwitchonE_MushroomColor (Variables|Default|GetE_Color)
    (:NewEnumerator0
      (Rendering|Components|Light|SetLightColor (Variables|Default|GetPointLight) "(R=1.000000,G=0.000000,B=0.701211,A=1.000000)" true))
    (:NewEnumerator1
      (Rendering|Components|Light|SetLightColor (Variables|Default|GetPointLight) "(R=1.000000,G=0.856120,B=0.000000,A=1.000000)" true))
    (:NewEnumerator2
      (Rendering|Components|Light|SetLightColor (Variables|Default|GetPointLight) "(R=0.000000,G=1.000000,B=0.967289,A=1.000000)" true))))

(event Custom|WRONG
  (Variables|Default|SetWrongAnime true)
  (Rendering|Components|Light|SetLightColor (Variables|Default|GetPointLight) "(R=1.000000,G=0.035759,B=0.000000,A=1.000000)" true)
  (Utilities|FlowControl|Delay 2.0)
  (CallFunction|SetColor)
  (Variables|Default|SetWrongAnime false))

(event Custom|Victory
  (Variables|Default|SetWiin true)
  (Rendering|Components|Light|SetLightColor (Variables|Default|GetPointLight) "(R=0.089220,G=1.000000,B=0.000000,A=1.000000)" true))

(event EventBeginPlay
  (CallFunction|SetColor))

(fn ConstructionScript)